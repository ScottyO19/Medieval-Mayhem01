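; Village objective capture point that announces when enemies or others enter or leave its Box trigger.
; Overlap events test whether a single AICharacter, found by GetActorOfClass, is inside, rather than checking the actor that triggered them.
; If it is on entry, a warning prints, then after a delay the Platform switches to the Knight material and the village is declared lost.
; End overlap only prints messages and does not cancel that pending loss.
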(event `self.ReceiveBeginPlay`)

(event `self.Box.OnComponentBeginOverlap`
  (params (OverlappedComponent :type "PrimitiveComponent Object Reference") (OtherActor :type "Actor Object Reference") (OtherComp :type "PrimitiveComponent Object Reference") (OtherBodyIndex :type Integer) (bFromSweep :type Boolean) (SweepResult :type "HitResult Structure (by ref)"))
  (bind _returnvalue (`GameplayStatics.GetActorOfClass` "/Game/AiCharacter/AICharacter.AICharacter_C"))
  (if (`PrimitiveComponent.IsOverlappingActor` OverlappedComponent _returnvalue)
    (`KismetSystemLibrary.PrintString` "The Enemeies are taking the village, stop them!")
    (`KismetSystemLibrary.Delay` 10.0)
    (`PrimitiveComponent.SetMaterial` (`self.Platform`) 0 "/Game/Multiplayer/Lobby/Characters/Temp_Materials/Knight.Knight")
    (`KismetSystemLibrary.PrintString` "The Village was lost, defend the Castle!")
    (else
      (`KismetSystemLibrary.PrintString` "You are on the objective!"))))

(event `self.Box.OnComponentEndOverlap`
  (params (OverlappedComponent :type "PrimitiveComponent Object Reference") (OtherActor :type "Actor Object Reference") (OtherComp :type "PrimitiveComponent Object Reference") (OtherBodyIndex :type Integer))
  (bind _returnvalue (`GameplayStatics.GetActorOfClass` "/Game/AiCharacter/AICharacter.AICharacter_C"))
  (if (`PrimitiveComponent.IsOverlappingActor` OverlappedComponent _returnvalue)
    (`KismetSystemLibrary.PrintString` "The Enemy is no longer on the objective!")
    (else
      (`KismetSystemLibrary.PrintString` "You have left the objective!"))))

(fn `UserConstructionScript`)